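; BP_PuzzleButton is a puzzle button that the third-person character presses by overlapping its trigger.
; BeginPlay creates a dynamic glowing material instance on the mesh.
; The first character overlap latches IsPressed, sets GlowAmount from the material's validity check converted to a number, and reports ButtonID to the puzzle manager.
; Nothing in this Blueprint resets the pressed state.
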(event `self.Button Trigger.OnComponentBeginOverlap`
  (params (OverlappedComponent :type "PrimitiveComponent Object Reference") (OtherActor :type "Actor Object Reference") (OtherComp :type "PrimitiveComponent Object Reference") (OtherBodyIndex :type Integer) (bFromSweep :type Boolean) (SweepResult :type "HitResult Structure (by ref)"))
  (bind _buttonmatref (`self.ButtonMatRef`))
  (cast `/Game/ThirdPerson/Blueprints/BP_ThirdPersonCharacter` OtherActor)
  (if (not (`self.IsPressed`))
    (set `self.IsPressed` true)
    (`MaterialInstanceDynamic.SetScalarParameterValue` _buttonmatref "GlowAmount" (`KismetMathLibrary.Conv_BoolToDouble` (`KismetSystemLibrary.IsValid` _buttonmatref)))
    (`/Game/Blueprints/BP_PuzzleManager.RegisterButtonPressed` (`self.PuzzleManagerRef`) (`self.ButtonID`))))

(event `self.ReceiveBeginPlay`
  (bind _returnvalue (`PrimitiveComponent.CreateDynamicMaterialInstance` (`self.StaticMesh`) 0 "/Game/Materials/M_GlowingButton.M_GlowingButton" "None"))
  (set `self.ButtonMatRef` _returnvalue))

(fn `UserConstructionScript`)